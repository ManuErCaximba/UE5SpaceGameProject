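; BP_SpacePlayerCharacter is a first-person player character that can move inside a ship's gravity field in space.
; While InGravityField, Tick zeroes gravity scale and mirrors CharacterCopy, mapping its offset from the ship copy's center of mass onto this CenterOfMass transform.
; It also combines rotations and copies the proxy's camera rotation, a proxy-simulation technique for local gravity.
; A rotate-player event pitches the actor 90 degrees and disables capsule gravity; its GameMode-guarded trigger is unconnected.
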(event Custom|RotatePlayer_Event
  (Transformation|SetActorRotation "0.000000,0.000000,90.000000")
  (Physics|SetEnableGravity (Variables|Default|GetCapsuleComponent) false))

(event EventTick
  (params (DeltaSeconds :type Float%20%28single-precision%29))
  (bind _charactercopy (Variables|Default|GetCharacterCopy))
  (bind _centerofmass (Variables|Default|GetCenterOfMass))
  (bind _returnvalue (Transformation|GetWorldTransform _centerofmass))
  (bind _returnvalue_2 (Transformation|GetActorTransform _charactercopy))
  (if (Variables|Default|GetbInGravityField)
    (Variables|/Script/Engine.CharacterMovementComponent|SetGravityScale (Variables|Character|GetCharacterMovement) 0.0)
    (Transformation|SetActorTransform (Math|Transform|MakeTransform (+ (.location _returnvalue) (Math|Vector|RotateVector (- (.location _returnvalue_2) (Transformation|GetWorldLocation (Variables|/Script/SpaceProject.SpaceShipVehicle|GetCenterOfMass (Variables|Default|GetShipCopyRef)))) (.rotation _returnvalue))) (Math|Rotator|CombineRotators (.rotation _returnvalue_2) (.rotation _returnvalue)) "1.000000,1.000000,1.000000"))
    (Transformation|SetRelativeRotation (Variables|Default|GetFirstPersonCameraComponent) (Variables|/Script/Engine.SceneComponent|GetRelativeRotation (Variables|/Script/SpaceProject.SpacePlayerCharacter|GetFirstPersonCameraComponent (Variables|Default|GetCharacterCopy))) false false)))

(event EventBeginPlay)

(fn ConstructionScript)