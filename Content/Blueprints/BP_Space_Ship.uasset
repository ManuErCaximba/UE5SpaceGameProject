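; Space ship actor that gives players local gravity by proxying them into a duplicate ship.
; On BeginPlay the server spawns a ship copy at a fixed transform.
; When a player character enters GravityBox, the server spawns a character copy in that ship, offset from CenterOfMass by the sweep impact point.
; The controller possesses the copy while the view stays on the original, which receives references to the copy, ship copy and CenterOfMass.
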(event OnComponentBeginOverlap(GravityBox)
  (params (OverlappedComponent :type Primitive%20Component%20Object%20Reference) (OtherActor :type Actor%20Object%20Reference) (OtherComp :type Primitive%20Component%20Object%20Reference) (OtherBodyIndex :type Integer) (bFromSweep :type Boolean) (SweepResult :type Hit%20Result%20Structure%20%28by%20ref%29))
  (bind _asbp_space_player_character (Utilities|Casting|CastToBP_SpacePlayerCharacter OtherActor))
  (if (and (not (Variables|/Game/Blueprints/BP_SpacePlayerCharacter.BP_SpacePlayerCharacter_C|GetbInGravityField _asbp_space_player_character)) (Ability|HasAuthority))
    (Variables|/Game/Blueprints/BP_SpacePlayerCharacter.BP_SpacePlayerCharacter_C|SetbInGravityField _asbp_space_player_character true)
    (bind _returnvalue (Game|SpawnActorfromClass "/Game/Blueprints/BP_SpacePlayerCharacter_Copy.BP_SpacePlayerCharacter_Copy_C" (Math|Transform|MakeTransform (- (.location (Transformation|GetWorldTransform (Variables|/Script/SpaceProject.SpaceShipVehicle|GetCenterOfMass (Variables|Default|GetShipCopyRef)))) (- (Transformation|GetWorldLocation (Variables|Default|GetCenterOfMass)) (.impactpoint SweepResult))) (.rotation (Transformation|GetWorldTransform (Variables|/Script/SpaceProject.SpaceShipVehicle|GetCenterOfMass (Variables|Default|GetShipCopyRef)))) (.scale (Transformation|GetWorldTransform (Variables|/Script/SpaceProject.SpaceShipVehicle|GetCenterOfMass (Variables|Default|GetShipCopyRef))))) "AdjustIfPossibleButAlwaysSpawn" "MultiplyWithRoot" 0 0))
    (bind _asplayer_controller (Utilities|Casting|CastToPlayerController (Pawn|GetController _asbp_space_player_character)))
    (Pawn|Possess (Pawn|GetController _asbp_space_player_character) _returnvalue)
    (Game|Player|SetViewTargetwithBlend _asplayer_controller _asbp_space_player_character 0.0 "VTBlend_Linear" 0.0 false)
    (Variables|/Game/Blueprints/BP_SpacePlayerCharacter.BP_SpacePlayerCharacter_C|SetCharacterCopy _asbp_space_player_character _returnvalue)
    (Variables|/Game/Blueprints/BP_SpacePlayerCharacter.BP_SpacePlayerCharacter_C|SetCenterOfMass _asbp_space_player_character (Variables|Default|GetCenterOfMass))
    (Variables|/Game/Blueprints/BP_SpacePlayerCharacter.BP_SpacePlayerCharacter_C|SetShipCopyRef _asbp_space_player_character (Variables|Default|GetShipCopyRef))))

(event EventBeginPlay
  (if (Ability|HasAuthority)
    (bind _returnvalue (Game|SpawnActorfromClass "/Game/Blueprints/BP_Space_Ship_Copy.BP_Space_Ship_Copy_C" (Math|Transform|MakeTransform "-1024.000000,-1690.000000,263.000000" "0.000000,0.000000,270.000000" "1.000000,1.000000,1.000000") "AlwaysSpawn" "MultiplyWithRoot" 0 0))
    (Variables|Default|SetShipCopyRef _returnvalue)))

(event EventTick
  (params (DeltaSeconds :type Float%20%28single-precision%29))
  (if (Ability|HasAuthority)
    _))

(fn ConstructionScript)